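; BP_GameMode is a game mode Blueprint that creates the HUD and tallies resources.
; On BeginPlay it creates WBP_HUD and adds it to the viewport.
; ResourceUp adds an amount to an existing key in Map1 and prints the value, ignoring missing keys.
; It assigns the sum through MakeMap, which replaces the whole map with that single entry, dropping any other keys.
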(event `self.ReceiveBeginPlay`
  (bind _returnvalue (`|CreateWidget` "/Game/Blueprints/Widgets/WBP_HUD.WBP_HUD_C"))
  (`UserWidget.AddToViewport` _returnvalue 0))

(event `ResourceUp`
  (params (NewParam :type String) (NewParam2 :type Integer))
  (bind (_value _returnvalue) (`BlueprintMapLibrary.Map_Find` (`self.Map1`) NewParam))
  (if _returnvalue
    (set `self.Map1` (`|MakeMap` NewParam (+ _value NewParam2)))
    (`KismetSystemLibrary.PrintString` (`KismetStringLibrary.Conv_IntToString` _value))))

(fn `UserConstructionScript`)